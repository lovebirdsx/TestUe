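; GA_Shoot is a Gameplay Ability that fires a bullet from the player character.
; On activation it casts the avatar to BP_Charactor and spawns a BP_Bullet at the Ammo socket, oriented to the camera's world rotation.
; A camera-rotated offset is added to the spawn location but is currently zero.
; The ability ends immediately after spawning; a failed cast stops execution without ending it.
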(event Ability|EventActivateAbility
  ;[0.05 0.05 0.05] Ability释放逻辑
  (bind _asbp_charactor (Utilities|Casting|CastToBP_Charactor (Ability|GetAvatarActorfromActorInfo)))
  (Game|SpawnActorfromClass "/Game/TestUe/Blueprints/BP_Bullet.BP_Bullet_C" (Math|Transform|MakeTransform (+ (Transformation|GetSocketLocation (Variables|/Game/TestUe/Blueprints/BP_Charactor.BP_Charactor_C|GetPlayer _asbp_charactor) "Ammo") (Math|Vector|RotateVector "0, 0, 0" (Transformation|GetWorldRotation (Variables|/Game/TestUe/Blueprints/BP_Charactor.BP_Charactor_C|GetCamera _asbp_charactor)))) (Transformation|GetWorldRotation (Variables|/Game/TestUe/Blueprints/BP_Charactor.BP_Charactor_C|GetCamera _asbp_charactor))) "Undefined" "OverrideRootScale" 0 0)
  (Ability|EndAbility))

(event Ability|EventOnEndAbility
  (params (bWasCancelled :type Boolean)))
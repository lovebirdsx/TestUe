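; BP_Bullet is a projectile actor that pushes physics objects and can set the hit actor on fire.
; On hit, it acts only if the struck component simulates physics, applying a velocity-scaled impulse at the bullet's location.
; It then applies the GE_LightOnFire gameplay effect through the hit actor's Ability System Component, if valid, and destroys itself.
; Hits on non-simulating components do nothing, leaving the bullet alive.
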(event Collision|EventHit
  (params (MyComp :type Primitive%20Component%20Object%20Reference) (Other :type Actor%20Object%20Reference) (OtherComp :type Primitive%20Component%20Object%20Reference) (bSelfMoved :type Boolean) (HitLocation :type Vector :default "0, 0, 0") (HitNormal :type Vector :default "0, 0, 0") (NormalImpulse :type Vector :default "0, 0, 0") (Hit :type Hit%20Result%20Structure%20%28by%20ref%29))
  (bind _returnvalue (Ability|GetAbilitySystemComponent Other))
  ;[0.15 0.15 0.15 0.5] 处理碰撞
  (if (Physics|IsSimulatingPhysics OtherComp "None")
    (Utilities|FlowControl|Sequence
      (:then_0
        (Physics|AddImpulseatLocation OtherComp (* (Transformation|GetVelocity) 1e+01) (Transformation|GetActorLocation) "None"))
      (:then_1
        (Utilities|IsValid _returnvalue
          (:Is%20Valid
            (GameplayEffects|ApplyGameplayEffectToSelf :self _returnvalue :GameplayEffectClass "/Game/TestUe/Blueprints/GE_LightOnFire.GE_LightOnFire_C"))))
      (:then_2
        (Actor|DestroyActor)))))

(fn ConstructionScript)
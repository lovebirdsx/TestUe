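; BP_MyActor is a test actor that shows the outermost object of its own instance and of its class.
; On BeginPlay it calls PrintOuterToScreen once with itself and once with its class, each with a label prefix.
; That function loops up the Outer chain until no valid outer remains, then prints only that last object's display name on screen.
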(event EventBeginPlay
  (CallFunction|PrintOutertoScreen "Self " self)
  (CallFunction|PrintOutertoScreen "Class " "BP_MyActor"))

(fn ConstructionScript)

(fn PrintOutertoScreen
  (params (Prefix :type String) (TempOuter :type Object%20Object%20Reference))
  (bind _output_get (Variables|Default|SetTempOuter TempOuter))
  (Utilities|IsValid (Utilities|GetOuterObject _output_get) :!label _label
    (:Is%20Valid
      (Variables|Default|SetTempOuter (Utilities|GetOuterObject _output_get))
      (goto _label))
    (:Is%20Not%20Valid
      (Development|PrintString (Utilities|String|Append Prefix (Utilities|GetDisplayName (Variables|Default|GetTempOuter))) true true "(R=0.000000,G=0.660000,B=1.000000,A=1.000000)" 2e+01))))
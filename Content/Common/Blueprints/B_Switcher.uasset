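; B_Switcher is a pressure-plate style trigger switch that turns a target on while pawns stand inside its box.
; On the authority, box overlaps count pawns entering and leaving, firing TriggerOn for the first entry and TriggerOff when the last leaves.
; Both functions print a debug message and forward the event to TriggerTarget through an interface, keeping the switch decoupled from what it controls.
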(event OnComponentBeginOverlap(Box)
  (params (OverlappedComponent :type Primitive%20Component%20Object%20Reference) (OtherActor :type Actor%20Object%20Reference) (OtherComp :type Primitive%20Component%20Object%20Reference) (OtherBodyIndex :type Integer) (bFromSweep :type Boolean) (SweepResult :type Hit%20Result%20Structure%20%28by%20ref%29))
  ;[0.15 0.15 0.15 0.5] 进入触发检测
  (if (Ability|HasAuthority)
    (bind _aspawn (Utilities|Casting|CastToPawn OtherActor))
    (bind _result (Math|Integer|IncrementInt (Variables|Default|GetOverlappedTargetCount))
      (:%20%20
        (bind _output_get (Variables|Default|SetOverlappedTargetCount _result))
        (if (== _output_get 1)
          (CallFunction|Triggeron _aspawn))))))

(event OnComponentEndOverlap(Box)
  (params (OverlappedComponent :type Primitive%20Component%20Object%20Reference) (OtherActor :type Actor%20Object%20Reference) (OtherComp :type Primitive%20Component%20Object%20Reference) (OtherBodyIndex :type Integer))
  ;[0.15 0.15 0.15 0.5] 退出触发检测
  (if (Ability|HasAuthority)
    (bind _aspawn (Utilities|Casting|CastToPawn OtherActor))
    (bind _result (Math|Integer|DecrementInt (Variables|Default|GetOverlappedTargetCount))
      (:%20%20
        (bind _output_get (Variables|Default|SetOverlappedTargetCount _result))
        (if (== _output_get 0)
          (CallFunction|TriggerOff _aspawn))))))

(fn ConstructionScript)

(fn Triggeron
  (params (Who :type Actor%20Object%20Reference))
  (bind _triggertarget (Variables|Default|GetTriggerTarget))
  (Development|PrintString (Utilities|String|Append "Trigger On By" (Utilities|GetDisplayName Who)))
  (if (Utilities|IsValidInterface _triggertarget)
    (Default|OnTriggeron _triggertarget)))

(fn TriggerOff
  (params (Who :type Actor%20Object%20Reference))
  (bind _triggertarget (Variables|Default|GetTriggerTarget))
  (Development|PrintString (Utilities|String|Append "Trigger Off By" (Utilities|GetDisplayName Who)))
  (if (Utilities|IsValidInterface _triggertarget)
    (Default|OnTriggerOff _triggertarget)))
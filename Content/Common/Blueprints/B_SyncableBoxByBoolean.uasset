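; Box actor that hops between two points on either side of its placed location along Y, kept in sync across the network through a single boolean.
; Trigger on/off events set IsMoving only with authority, while Tick toggles the position every second as long as it is true.
; Its OnRep resets the timer and snaps the box to the first point on start, aligning each machine's locally run motion.
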(event EventTick
  (params (DeltaSeconds :type Float%20%28single-precision%29))
  (if (Variables|Default|GetIsMoving)
    (bind _output_get (Variables|Default|SetTimeCounter (+ DeltaSeconds (Variables|Default|GetTimeCounter))))
    (if (>= _output_get 1.0)
      (Variables|Default|SetTimeCounter (- (Variables|Default|GetTimeCounter) 1.0))
      (CallFunction|TriggleLocation))))

(event EventOnTriggerOff
  (if (Ability|HasAuthority)
    (Variables|Default|SetIsMoving false)))

(event EventOnTriggeron
  (if (Ability|HasAuthority)
    (Variables|Default|SetIsMoving true)))

(fn ConstructionScript
  (bind _returnvalue (Transformation|GetActorLocation))
  (Variables|Default|SetP1 (+ _returnvalue "0.000000,100.000000,0.000000"))
  (Variables|Default|SetP2 (+ _returnvalue "0.000000,-100.000000,0.000000")))

(fn OnRepIsMoving
  (if (Variables|Default|GetIsMoving)
    (Variables|Default|SetTimeCounter 0.0)
    (Transformation|SetActorLocation (Variables|Default|GetP1) false false)))

(fn TriggleLocation
  (if (> (Math|Vector|Distance2D(Vector) (Math|Conversions|ToVector2D(Vector) (Transformation|GetActorLocation)) (Math|Conversions|ToVector2D(Vector) (Variables|Default|GetP1))) 1e+02)
    (Transformation|SetActorLocation (Variables|Default|GetP1) false false)
    (else
      (Transformation|SetActorLocation (Variables|Default|GetP2) false false))))
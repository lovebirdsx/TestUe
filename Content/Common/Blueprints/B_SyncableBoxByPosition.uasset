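; Replicated box actor that moves back and forth along world Y between two points 100 units either side of its construction location.
; On authority, Tick advances a position by the start-to-target vector times Speed, reversing on overshoot or near arrival.
; The RepNotify on Pos applies the location directly, syncing movement without interpolation.
; The construction script sets the endpoints and a configurable NetUpdateFrequency.
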(event EventTick
  (params (DeltaSeconds :type Float%20%28single-precision%29))
  (if (Ability|HasAuthority)
    (if (or (< (Class|KismetMathLibrary|VectorDistanceSquared (Variables|Default|GetTargetPos) (Variables|Default|GetStartPos)) (Class|KismetMathLibrary|VectorDistanceSquared (Variables|Default|GetStartPos) (+ (* DeltaSeconds (* (- (Variables|Default|GetTargetPos) (Variables|Default|GetStartPos)) (Variables|Default|GetSpeed))) (Transformation|GetActorLocation)))) (< (Class|KismetMathLibrary|VectorDistanceSquared (+ (* DeltaSeconds (* (- (Variables|Default|GetTargetPos) (Variables|Default|GetStartPos)) (Variables|Default|GetSpeed))) (Transformation|GetActorLocation)) (Variables|Default|GetTargetPos)) 1e+01))
      (if (< (Class|KismetMathLibrary|VectorDistanceSquared (Variables|Default|GetTargetPos) (Variables|Default|GetStartPos)) (Class|KismetMathLibrary|VectorDistanceSquared (Variables|Default|GetStartPos) (+ (* DeltaSeconds (* (- (Variables|Default|GetTargetPos) (Variables|Default|GetStartPos)) (Variables|Default|GetSpeed))) (Transformation|GetActorLocation))))
        (Variables|Default|SetPos (Variables|Default|GetTargetPos))
        (else
          (Variables|Default|SetPos (+ (* DeltaSeconds (* (- (Variables|Default|GetTargetPos) (Variables|Default|GetStartPos)) (Variables|Default|GetSpeed))) (Transformation|GetActorLocation)))))
      ;[0.15 0.15 0.15 0.5] 朝另外一个方向移动
      (if (< (Class|KismetMathLibrary|VectorDistanceSquared (Variables|Default|GetTargetPos) (Variables|Default|GetP1)) 1e+01)
        (Variables|Default|SetStartPos (Variables|Default|GetP1))
        (Variables|Default|SetTargetPos (Variables|Default|GetP2))
        (else
          (Variables|Default|SetStartPos (Variables|Default|GetP2))
          (Variables|Default|SetTargetPos (Variables|Default|GetP1))))
      (else
        (Variables|Default|SetPos (+ (* DeltaSeconds (* (- (Variables|Default|GetTargetPos) (Variables|Default|GetStartPos)) (Variables|Default|GetSpeed))) (Transformation|GetActorLocation)))))))

(fn ConstructionScript
  (bind _returnvalue (Transformation|GetActorLocation))
  (bind _returnvalue_2 (+ _returnvalue "0.000000,100.000000,0.000000"))
  (Utilities|FlowControl|Sequence
    (:then_0
      ;[0.15 0.15 0.15 0.5] 初始化相关位置
      (Variables|Default|SetP1 _returnvalue_2)
      (Variables|Default|SetP2 (+ _returnvalue "0.000000,-100.000000,0.000000"))
      (Variables|Default|SetTargetPos _returnvalue_2)
      (Variables|Default|SetStartPos _returnvalue))
    (:then_1
      (Variables|Default|SetNetUpdateFrequency (Variables|Default|GetUpdateFrequency)))))

(fn OnRepPos
  (Transformation|SetActorLocation (Variables|Default|GetPos) false false))
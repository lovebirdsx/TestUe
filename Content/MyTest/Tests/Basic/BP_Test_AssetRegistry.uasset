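; Functional test that checks Asset Registry queries from Blueprint against sample assets under /Game/MyTest.
; On start it runs four checks in sequence, then finishes as Succeeded.
; Lookups by path, class (including subclasses) and package name assert on result counts.
; The object-path lookup verifies individual asset data fields, expecting AssetClass to be None and AssetClassPath to identify a Blueprint.
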(event EventStartTest
  (CallFunction|TestGetAssetbyPath)
  (CallFunction|TestGetAssetsbyClass)
  (CallFunction|TestGetAssetsbyPackageName)
  (CallFunction|TestGetAssetbyObjectPath)
  (Class|FunctionalTest|FinishTest "Succeeded"))

(fn ConstructionScript)

(fn TestGetAssetbyPath
  (bind _outassetdata (Class|AssetRegistry|GetAssetsbyPath (Class|AssetRegistryHelpers|GetAssetRegistry) "/Game/MyTest" true true))
  (Class|FunctionalTest|AssertValueInt (Utilities|Array|Length _outassetdata) "Greater_Than" 0 "GetAssetsByPath"))

(fn TestGetAssetsbyClass
  (bind _outassetdata (Class|AssetRegistry|GetAssetsbyClass (Class|AssetRegistryHelpers|GetAssetRegistry) (Utilities|MakeTopLevelAssetPath "/Script/MyAsset" "MyCustomAsset2") true))
  (Class|FunctionalTest|AssertValueInt (Utilities|Array|Length _outassetdata) "Greater_Than" 0 "GetAssetsByClass"))

(fn TestGetAssetsbyPackageName
  (bind _outassetdata (Class|AssetRegistry|GetAssetsbyPackageName (Class|AssetRegistryHelpers|GetAssetRegistry) "/Game/MyTest/BP_MyObject1" true true))
  (Class|FunctionalTest|AssertValueInt (Utilities|Array|Length _outassetdata) "Greater_Than" 0 "GetAssetByPackageName"))

(fn TestGetAssetbyObjectPath
  (bind _returnvalue (Class|AssetRegistry|GetAssetbyObjectPath (Class|AssetRegistryHelpers|GetAssetRegistry) (Utilities|MakeSoftObjectPath "/Game/MyTest/BP_MyObject1.BP_MyObject1") true true))
  (Class|FunctionalTest|AssertTrue (Class|AssetRegistryHelpers|IsValid _returnvalue) "GetAssetByObjectPath")
  (Class|FunctionalTest|AssertEqualName (.PackageName (Utilities|Struct|BreakAssetData _returnvalue)) "/Game/MyTest/BP_MyObject1" "Package Name")
  (Class|FunctionalTest|AssertEqualName (.PackagePath (Utilities|Struct|BreakAssetData _returnvalue)) "/Game/MyTest" "Package Path")
  (Class|FunctionalTest|AssertEqualName (.AssetName (Utilities|Struct|BreakAssetData _returnvalue)) "BP_MyObject1" "Asset Name")
  (Class|FunctionalTest|AssertEqualName (.AssetClass (Utilities|Struct|BreakAssetData _returnvalue)) "None" "Asset Class")
  (Class|FunctionalTest|AssertEqualString (Class|KismetSystemLibrary|BreakTopLevelAssetPath (.AssetClassPath (Utilities|Struct|BreakAssetData _returnvalue))) "/Script/Engine.Blueprint" "Asset Class Path"))